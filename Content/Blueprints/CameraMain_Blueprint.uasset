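; Main camera actor that scrolls vertically upward through the level until it reaches an end height.
; BeginPlay teleports it to StartPos.
; While IsMoving is set, each Tick raises it along Z by ScrollSpeed scaled by world delta time, using a swept move.
; Tick first clears IsMoving once Z reaches or passes EndZ, and nothing here sets it again.
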(event `self.ReceiveBeginPlay`
  (`self.K2_SetActorLocation` (`self.startPos`) false true))

(event `self.ReceiveTick`
  (params (DeltaSeconds :type "Float (single-precision)"))
  (`|ExecutionSequence`
    (:`then_0`
      ;[1 1 1] Check for stop movement
      (`/Engine/EditorBlueprintResources/StandardMacros.CompareFloat` (.z (`self.K2_GetActorLocation`)) (`self.endZ`)
        (:`>`
          _)
        (:`==`
          _))
      (set `self.isMoving` false))
    (:`then_1`
      (if (`self.isMoving`)
        ;[1 1 1] Vertical Scroll
        (`self.K2_SetActorLocation` (+ (`self.K2_GetActorLocation`) (* (0.0 0.0 1.0) (* (`GameplayStatics.GetWorldDeltaSeconds`) (`self.scrollSpeed`)))) true)))))

(fn `UserConstructionScript`)